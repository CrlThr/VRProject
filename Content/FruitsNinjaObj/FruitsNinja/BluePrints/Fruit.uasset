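; Fruit actor for a Fruit Ninja-style game that the player slices with a sword for score.
; It destroys itself on a short timer after BeginPlay, so missed fruit is cleaned up as it falls.
; A hit from an actor tagged Sword plays a cut sound, calls AddFruits on the Score_FN widget found through BP_Counter's widget component, then destroys the fruit.
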(event `self.ReceiveBeginPlay`
  ; fruits will detroy after falling
  (`KismetSystemLibrary.Delay` 2.5)
  (`self.K2_DestroyActor`))

(event `self.ReceiveHit`
  (params (MyComp :type "PrimitiveComponent Object Reference") (Other :type "Actor Object Reference") (OtherComp :type "PrimitiveComponent Object Reference") (bSelfMoved :type Boolean) (HitLocation :type "Vector Structure") (HitNormal :type "Vector Structure") (NormalImpulse :type "Vector Structure") (Hit :type "HitResult Structure (by ref)"))
  ; if you hit the fruit with sword, play a sound effet
  (if (`self.ActorHasTag` Other "Sword")
    (`GameplayStatics.PlaySoundAtLocation` "/Game/FruitsNinjaObj/FruitsNinja/cyberwave-orchestra-fantasy-game-sword-cut-sound-effect-get-more-on-my-patreon-339824.cyberwave-orchestra-fantasy-game-sword-cut-sound-effect-get-more-on-my-patreon-339824" HitLocation (struct) 1.0 1.0 0.0 null null null null)
    ; increment score and destroy the fruit
    (bind _returnvalue (`GameplayStatics.GetActorOfClass` "/Game/FruitsNinjaObj/FruitsNinja/BluePrints/BP_Counter.BP_Counter_C"))
    (bind _asscore_fn (cast `/Game/FruitsNinjaObj/FruitsNinja/Score_FN` (`WidgetComponent.GetUserWidgetObject` (`/Game/FruitsNinjaObj/FruitsNinja/BluePrints/BP_Counter.Widget` _returnvalue))))
    (`/Game/FruitsNinjaObj/FruitsNinja/Score_FN.AddFruits` _asscore_fn)
    (`self.K2_DestroyActor`)))

(fn `UserConstructionScript`)