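; Spawner actor for a Fruit Ninja style level that keeps tossing fruits and bombs into the air.
; From BeginPlay, LaunchWave spawns a weighted random Bomb or Fruit at a random point inside its Box bounds, rotated to match and offset to the box location.
; It launches the spawned mesh upward with a random velocity-change impulse, then reschedules itself after a random delay.
; An unused looping timer alternative is left disconnected.
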(event `LaunchWave`
  (bind _box (`self.Box`))
  (bind _returnvalue (`|SpawnActorFromClass` (select `bool` (`KismetMathLibrary.RandomBoolWithWeight` 0.3) :`false` "/Game/Level/FruitsNinja/BluePrints/Fruit.Fruit_C" :`true` "/Game/Level/FruitsNinja/BluePrints/Bomb.Bomb_C" :!type "Actor Class Reference") (`KismetMathLibrary.MakeTransform` (+ (`KismetMathLibrary.RotateAngleAxis` (`KismetMathLibrary.RandomPointInBoundingBox` (0.0 0.0 0.0) (`BoxComponent.GetScaledBoxExtent` _box)) 90.0 (0.0 0.0 1.0)) (`SceneComponent.K2_GetComponentLocation` _box))) "Undefined" "MultiplyWithRoot" null null))
  (`PrimitiveComponent.AddImpulse` (`self.GetComponentByClass` _returnvalue "/Script/Engine.StaticMeshComponent") (`KismetMathLibrary.MakeVector` 0.0 0.0 (`KismetMathLibrary.RandomFloatInRange` 530.0 580.0)) "None" true)
  (`KismetSystemLibrary.Delay` (`KismetMathLibrary.RandomFloatInRange` 0.7 2.0))
  (`self.LaunchWave`))

(event `self.ReceiveBeginPlay`
  ; spawning waves
  (`self.LaunchWave`))

(fn `UserConstructionScript`)