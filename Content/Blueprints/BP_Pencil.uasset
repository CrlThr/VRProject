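; Pencil actor that paints brush strokes onto a BP_Canvas when its nib is close enough to touch it.
; Each Tick, a long forward trace finds the canvas hit UV, and a short trace sets IsDrawing for the following frame.
; While drawing, it calls the canvas's DrawBrush at interpolated UV steps between previous and current positions to fill gaps.
; An older copy of this logic remains disabled in a custom event.
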(event `self.ReceiveTick`
  (params (DeltaSeconds :type "Float (single-precision)"))
  (bind _returnvalue (`self.K2_GetActorLocation`))
  (bind _returnvalue_2 (`self.K2_GetActorLocation`))
  (`|ExecutionSequence`
    (:`then_0`
      ; Constantly update CurrentPos and PreviousPos, Draws if IsDrawing True
      (bind _outhit (`KismetSystemLibrary.LineTraceSingle` :`Start` _returnvalue :`End` (+ _returnvalue (* (`SceneComponent.GetForwardVector` (`self.PencilMesh`)) 1500.0)) :`TraceChannel` "TraceTypeQuery1" :`bTraceComplex` true :`TraceColor` (struct :`R` 1.0 :`G` 0.785191 :`A` 1.0)))
      (bind _asbp_canvas (cast `/Game/Blueprints/BP_Canvas` (`.HitActor` (`GameplayStatics.BreakHitResult` _outhit))))
      (bind _output_get (set `self.CurrentPos` (`GameplayStatics.FindCollisionUV` _outhit)))
      (bind _returnvalue_3 (`KismetMathLibrary.Conv_Int64ToInt` (`KismetMathLibrary.Conv_DoubleToInt64` (* (`KismetMathLibrary.Distance2D` _output_get (`self.PreviousPos`)) 1024.0))))
      (for _index (range (+ _returnvalue_3 1))
        (if (`self.IsDrawing`)
          (`/Game/Blueprints/BP_Canvas.DrawBrush` _asbp_canvas (`self.BrushTexture`) (`self.BrushSize`) (+ (* (/ (- (`self.PreviousPos`) (`self.CurrentPos`)) (`KismetMathLibrary.MakeVector2D` (`KismetMathLibrary.Conv_IntToDouble` _returnvalue_3) (`KismetMathLibrary.Conv_IntToDouble` _returnvalue_3))) (`KismetMathLibrary.MakeVector2D` (`KismetMathLibrary.Conv_IntToDouble` _index) (`KismetMathLibrary.Conv_IntToDouble` _index))) (`self.CurrentPos`)))))
      (set `self.PreviousPos` (`self.CurrentPos`)))
    (:`then_1`
      ; Detect with Second Line trace to make True if pencil nib is touching the Canva
      (bind _outhit_2 (`KismetSystemLibrary.LineTraceSingle` :`Start` _returnvalue_2 :`End` (+ _returnvalue_2 (* (`SceneComponent.GetForwardVector` (`self.PencilMesh`)) 16.0)) :`TraceChannel` "TraceTypeQuery1" :`bTraceComplex` true :`DrawDebugType` "ForOneFrame"))
      (if (== (`GameplayStatics.GetObjectClass` (`.HitActor` (`GameplayStatics.BreakHitResult` _outhit_2))) "/Game/Blueprints/BP_Canvas.BP_Canvas_C")
        (set `self.IsDrawing` true)
        (else
          (set `self.IsDrawing` false))))))

(fn `UserConstructionScript`)