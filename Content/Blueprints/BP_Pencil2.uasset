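; Pencil actor that paints on a BP_DrawingSurface it points at, using the hit point's collision UV.
; Each Tick, a long visibility trace along the mesh's forward vector calls DrawBrush with a fixed size, regardless of nib contact.
; An unconnected older path targets BP_Canvas, interpolating strokes between previous and current UVs and using a short nib trace to set IsDrawing; it never runs.
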(event `self.ReceiveTick`
  (params (DeltaSeconds :type "Float (single-precision)"))
  (bind _returnvalue (`self.K2_GetActorLocation`))
  (bind _outhit (`KismetSystemLibrary.LineTraceSingle` :`Start` _returnvalue :`End` (+ _returnvalue (* (`SceneComponent.GetForwardVector` (`self.PencilMesh`)) 1500.0)) :`TraceChannel` "TraceTypeQuery1" :`bTraceComplex` true :`DrawDebugType` "ForOneFrame" :`TraceColor` (struct :`R` 1.0 :`G` 0.785191 :`A` 1.0)))
  (bind _asbp_drawing_surface (cast `/Game/Blueprints/BP_DrawingSurface` (`.HitActor` (`GameplayStatics.BreakHitResult` _outhit))))
  (`/Game/Blueprints/BP_DrawingSurface.DrawBrush` _asbp_drawing_surface 10.0 (`GameplayStatics.FindCollisionUV` _outhit)))

(fn `UserConstructionScript`)