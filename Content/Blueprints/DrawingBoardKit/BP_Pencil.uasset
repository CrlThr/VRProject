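; Pencil actor that draws on a BP_Canvas while its nib is touching the surface.
; Each tick, a long forward trace from PencilMesh reads the canvas collision UV and, while IsDrawing, stamps DrawBrush at interpolated points back to the previous UV to keep strokes continuous.
; A second, short trace then sets IsDrawing according to whether it hits the canvas, so drawing uses the previous tick's contact state.
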(event `self.ReceiveTick`
  (params (DeltaSeconds :type "Float (single-precision)"))
  (`|ExecutionSequence`
    (:`then_0`
      ; Constantly update CurrentPos and PreviousPos, Draws if IsDrawing True
      (bind (_start _end) (`self.MeshPoint` 1500.0))
      (bind _outhit (`KismetSystemLibrary.LineTraceSingle` :`Start` _start :`End` _end :`TraceChannel` "TraceTypeQuery1" :`bTraceComplex` true :`TraceColor` (struct :`R` 1.0 :`G` 0.785191 :`A` 1.0)))
      (bind _asbp_canvas (cast `/Game/Blueprints/DrawingBoardKit/BP_Canvas` (`.HitActor` (`GameplayStatics.BreakHitResult` _outhit))))
      (bind _output_get (set `self.CurrentPos` (`GameplayStatics.FindCollisionUV` _outhit)))
      (bind _returnvalue (`KismetMathLibrary.Conv_Int64ToInt` (`KismetMathLibrary.Conv_DoubleToInt64` (* (`KismetMathLibrary.Distance2D` _output_get (`self.PreviousPos`)) 1024.0))))
      (for _index (range (+ _returnvalue 1))
        (if (`self.IsDrawing`)
          (`/Game/Blueprints/DrawingBoardKit/BP_Canvas.DrawBrush` _asbp_canvas (`self.BrushTexture`) (`self.BrushSize`) (+ (* (/ (- (`self.PreviousPos`) (`self.CurrentPos`)) (`KismetMathLibrary.MakeVector2D` (`KismetMathLibrary.Conv_IntToDouble` _returnvalue) (`KismetMathLibrary.Conv_IntToDouble` _returnvalue))) (`KismetMathLibrary.MakeVector2D` (`KismetMathLibrary.Conv_IntToDouble` _index) (`KismetMathLibrary.Conv_IntToDouble` _index))) (`self.CurrentPos`)))))
      (set `self.PreviousPos` (`self.CurrentPos`)))
    (:`then_1`
      ; Detect with Second Line trace to make True if pencil nib is touching the Canva
      (bind (_start_2 _end_2) (`self.MeshPoint` 16.0))
      (bind _outhit_2 (`KismetSystemLibrary.LineTraceSingle` :`Start` _start_2 :`End` _end_2 :`TraceChannel` "TraceTypeQuery1" :`bTraceComplex` true :`DrawDebugType` "ForOneFrame"))
      (if (== (`GameplayStatics.GetObjectClass` (`.HitActor` (`GameplayStatics.BreakHitResult` _outhit_2))) "/Game/Blueprints/DrawingBoardKit/BP_Canvas.BP_Canvas_C")
        (set `self.IsDrawing` true)
        (else
          (set `self.IsDrawing` false))))))

(fn `MeshPoint`
  (params (InteractionRange :type "Float (double-precision)"))
  (returns (Start :type "Vector Structure") (End :type "Vector Structure"))
  (bind _pencilmesh (`self.PencilMesh`))
  (bind _returnvalue (`SceneComponent.K2_GetComponentLocation` _pencilmesh))
  (return _returnvalue (+ _returnvalue (* (`SceneComponent.GetForwardVector` _pencilmesh) InteractionRange))))

(fn `UserConstructionScript`)