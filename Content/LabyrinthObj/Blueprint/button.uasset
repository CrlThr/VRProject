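; A labyrinth pressure button that opens the way by destroying a Door actor when the VR player presses it.
; When a VRPawn overlaps the Box, ButtonInteract sinks slightly and a sound plays, using the component's relative position as the world location.
; The Door is found by class lookup rather than a set reference.
; Ending the overlap raises the button to its stored start position, while the Door stays destroyed.
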(event `self.ReceiveBeginPlay`
  (set `self.Relative Location` (`SceneComponent.RelativeLocation` (`self.ButtonInteract`))))

(event `self.Box.OnComponentBeginOverlap`
  (params (OverlappedComponent :type "PrimitiveComponent Object Reference") (OtherActor :type "Actor Object Reference") (OtherComp :type "PrimitiveComponent Object Reference") (OtherBodyIndex :type Integer) (bFromSweep :type Boolean) (SweepResult :type "HitResult Structure (by ref)"))
  (bind _returnvalue (- (`self.Relative Location`) (0.0 0.0 5.0)))
  (cast `/Game/VRTemplate/Blueprints/VRPawn` OtherActor)
  (`KismetSystemLibrary.MoveComponentTo` (`self.ButtonInteract`) _returnvalue (struct) false false 0.1)
  (`GameplayStatics.PlaySoundAtLocation` "/Game/LabyrinthObj/3DObjects/buttonSound.buttonSound" _returnvalue (struct) 1.0 1.0 0.0 null null null null)
  (bind _returnvalue_2 (`GameplayStatics.GetActorOfClass` "/Game/LabyrinthObj/Blueprint/Door.Door_C"))
  (`self.K2_DestroyActor` _returnvalue_2))

(event `self.Box.OnComponentEndOverlap`
  (params (OverlappedComponent :type "PrimitiveComponent Object Reference") (OtherActor :type "Actor Object Reference") (OtherComp :type "PrimitiveComponent Object Reference") (OtherBodyIndex :type Integer))
  (cast `/Game/VRTemplate/Blueprints/VRPawn` OtherActor)
  (`KismetSystemLibrary.MoveComponentTo` (`self.ButtonInteract`) (`self.Relative Location`) (struct) false false 0.1))

(fn `UserConstructionScript`)