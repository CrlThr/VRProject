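; Night is a trigger volume in the labyrinth that switches lighting toward night when the player's VR pawn overlaps its Box.
; Entering plays a Timeline whose updates set intensity on the DayLight and NightLight references.
; Leaving reverses the Timeline, but both Lerps use constant alphas, so every update writes the same dimmed-day and faint-night levels instead of fading or restoring daylight.
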(event `self.Box.OnComponentBeginOverlap`
  (params (OverlappedComponent :type "PrimitiveComponent Object Reference") (OtherActor :type "Actor Object Reference") (OtherComp :type "PrimitiveComponent Object Reference") (OtherBodyIndex :type Integer) (bFromSweep :type Boolean) (SweepResult :type "HitResult Structure (by ref)"))
  (bind _asvrpawn (cast `/Game/VRTemplate/Blueprints/VRPawn` (`GameplayStatics.GetPlayerPawn` 0)))
  (if (== _asvrpawn OtherActor)
    (`Timeline|Timeline` :!label _label
      (:`Update`
        (`LightComponent.SetIntensity` (`Light.LightComponent` (`self.DayLight`)) (`KismetMathLibrary.Lerp` 2.0 0.0 0.5))
        (`LightComponent.SetIntensity` (`Light.LightComponent` (`self.NightLight`)) (`KismetMathLibrary.Lerp` 0.0 0.5 0.1))))))

(event `self.Box.OnComponentEndOverlap`
  (params (OverlappedComponent :type "PrimitiveComponent Object Reference") (OtherActor :type "Actor Object Reference") (OtherComp :type "PrimitiveComponent Object Reference") (OtherBodyIndex :type Integer))
  (bind _asvrpawn (cast `/Game/VRTemplate/Blueprints/VRPawn` (`GameplayStatics.GetPlayerPawn` 0)))
  (if (== _asvrpawn OtherActor)
    (goto _label :!via `Reverse`)))

(fn `UserConstructionScript`)